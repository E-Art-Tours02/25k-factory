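; Test water actor that exists visibly and physically only while the player is in the InterWorld state.
; BeginPlay caches the BP_PlayerState actor, and Tick reads its InterWorld flag to toggle the Sphere's visibility and collision.
; Tick also nudges the actor upward by a fixed, frame-rate-dependent step, whatever the world state.
; AI move, component move and delayed-show experiments remain unconnected, and testMove is empty.
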(event `self.ReceiveBeginPlay`
  (bind _returnvalue (`GameplayStatics.GetActorOfClass` "/Game/Blueprints/BP_PlayerState.BP_PlayerState_C"))
  (set `self.playerState_` _returnvalue))

(event `self.ReceiveTick`
  (params (DeltaSeconds :type "Float (single-precision)"))
  (bind (_returnvalue_x _returnvalue_y _returnvalue_z) (`KismetMathLibrary.BreakVector` (`self.K2_GetActorLocation`)))
  (bind _sphere (`self.Sphere`))
  (bind _sphere_2 (`self.Sphere`))
  (`self.K2_SetActorLocation` (`KismetMathLibrary.MakeVector` _returnvalue_x _returnvalue_y (+ _returnvalue_z 0.1)))
  (bind _output_get (set `self.Interworld` (`/Game/Blueprints/BP_PlayerState.InterWorld` (`self.playerState_`))))
  (if _output_get
    (`SceneComponent.SetHiddenInGame` _sphere_2 false false)
    (`PrimitiveComponent.SetCollisionEnabled` _sphere_2 "QueryAndPhysics")
    (else
      (`SceneComponent.SetHiddenInGame` _sphere true false)
      (`PrimitiveComponent.SetCollisionEnabled` _sphere "NoCollision") ; changement de LOD aussi ?
    )))

(event `testMove`)

(fn `UserConstructionScript`)