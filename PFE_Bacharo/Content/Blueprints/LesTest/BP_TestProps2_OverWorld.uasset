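; BP_TestProps2_OverWorld is a test prop whose sphere is present only while the player is outside the InterWorld.
; BeginPlay finds the BP_PlayerState actor and caches it.
; Tick polls its InterWorld flag every frame, hiding the sphere and disabling its collision when true, and restoring visibility with query and physics collision when false.
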(event `self.ReceiveBeginPlay`
  (bind _returnvalue (`GameplayStatics.GetActorOfClass` "/Game/Blueprints/BP_PlayerState.BP_PlayerState_C"))
  (set `self.PlayerState` _returnvalue))

(event `self.ReceiveTick`
  (params (DeltaSeconds :type "Float (single-precision)"))
  (bind _sphere (`self.Sphere`))
  (bind _sphere_2 (`self.Sphere`))
  (bind _output_get (set `self.Interworld` (`/Game/Blueprints/BP_PlayerState.InterWorld` (`self.PlayerState`))))
  (if _output_get
    (`SceneComponent.SetHiddenInGame` _sphere true false)
    (`PrimitiveComponent.SetCollisionEnabled` _sphere "NoCollision")
    (else
      (`SceneComponent.SetHiddenInGame` _sphere_2 false false)
      (`PrimitiveComponent.SetCollisionEnabled` _sphere_2 "QueryAndPhysics"))))

(fn `UserConstructionScript`)