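; Test actor that shows a particle effect (NSTest1) when the player is nearby and in the InterWorld state.
; A sphere trigger flags overlap by actors tagged "Player"; while overlapping, Tick polls InterWorld on the BP_PlayerState found at BeginPlay and activates the effect.
; The effect is deactivated only when the player exits the sphere, not when InterWorld turns false.
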(event `self.ReceiveBeginPlay`
  (bind _returnvalue (`GameplayStatics.GetActorOfClass` "/Game/Blueprints/BP_PlayerState.BP_PlayerState_C"))
  (set `self.PlayerState` _returnvalue))

(event `self.ReceiveTick`
  (params (DeltaSeconds :type "Float (single-precision)"))
  (if (`self.isOverlaping`)
    (bind _output_get (set `self.Inter World` (`/Game/Blueprints/BP_PlayerState.InterWorld` (`self.PlayerState`))))
    (if _output_get
      (`ActorComponent.Activate` (`self.NS_Test1`) false))))

(event `self.Sphere.OnComponentBeginOverlap`
  (params (OverlappedComponent :type "PrimitiveComponent Object Reference") (OtherActor :type "Actor Object Reference") (OtherComp :type "PrimitiveComponent Object Reference") (OtherBodyIndex :type Integer) (bFromSweep :type Boolean) (SweepResult :type "HitResult Structure (by ref)"))
  (if (`self.ActorHasTag` OtherActor "Player")
    (`KismetSystemLibrary.PrintString` "Player enter")
    (set `self.isOverlaping` true)))

(event `self.Sphere.OnComponentEndOverlap`
  (params (OverlappedComponent :type "PrimitiveComponent Object Reference") (OtherActor :type "Actor Object Reference") (OtherComp :type "PrimitiveComponent Object Reference") (OtherBodyIndex :type Integer))
  (if (`self.ActorHasTag` OtherActor "Player")
    (`ActorComponent.SetActive` (`self.NS_Test1`) false false)
    (set `self.isOverlaping` false)))

(fn `UserConstructionScript`)