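; Test prop whose Sphere changes its material look according to whether the player is in the InterWorld.
; On BeginPlay it finds and caches the BP_PlayerState actor.
; Every Tick it polls that InterWorld flag, calls CreateDynamicMaterialInstance on the Sphere's first material slot, and snaps the Alpha_Lerp_Textures parameter to one end of the texture blend or the other.
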(event `self.ReceiveBeginPlay`
  (bind _returnvalue (`GameplayStatics.GetActorOfClass` "/Game/Blueprints/BP_PlayerState.BP_PlayerState_C"))
  (set `self.PlayerState` _returnvalue))

(event `self.ReceiveTick`
  (params (DeltaSeconds :type "Float (single-precision)"))
  (bind _sphere (`self.Sphere`))
  (bind _sphere_2 (`self.Sphere`))
  (bind _output_get (set `self.Interworld` (`/Game/Blueprints/BP_PlayerState.InterWorld` (`self.PlayerState`))))
  (if _output_get
    (bind _returnvalue (`PrimitiveComponent.CreateDynamicMaterialInstance` _sphere_2 0 (`PrimitiveComponent.GetMaterial` _sphere_2 0) "None"))
    (`MaterialInstanceDynamic.SetScalarParameterValue` _returnvalue "Alpha_Lerp_Textures" 0.0)
    (else
      (bind _returnvalue_2 (`PrimitiveComponent.CreateDynamicMaterialInstance` _sphere 0 (`PrimitiveComponent.GetMaterial` _sphere 0) "None"))
      (`MaterialInstanceDynamic.SetScalarParameterValue` _returnvalue_2 "Alpha_Lerp_Textures" 1.0))))

(fn `UserConstructionScript`)