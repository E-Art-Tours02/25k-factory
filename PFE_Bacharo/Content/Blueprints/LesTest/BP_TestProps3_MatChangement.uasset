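; BP_TestProps3_MatChangement is a test prop whose sphere changes material to match the player's current world state.
; On BeginPlay it finds and caches the BP_PlayerState actor.
; Every Tick it polls that state's InterWorld flag and sets the Sphere's first material slot to either the InterWorld or OverWorld material, with no change detection.
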(event `self.ReceiveBeginPlay`
  (bind _returnvalue (`GameplayStatics.GetActorOfClass` "/Game/Blueprints/BP_PlayerState.BP_PlayerState_C"))
  (set `self.PlayerState` _returnvalue))

(event `self.ReceiveTick`
  (params (DeltaSeconds :type "Float (single-precision)"))
  (bind _output_get (set `self.Interworld` (`/Game/Blueprints/BP_PlayerState.InterWorld` (`self.PlayerState`))))
  (if _output_get
    (`PrimitiveComponent.SetMaterial` (`self.Sphere`) 0 (`self.matInterWorld`))
    (else
      (`PrimitiveComponent.SetMaterial` (`self.Sphere`) 0 (`self.matOverWorld`)))))

(fn `UserConstructionScript`)